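; First-person player character with two arm weapon slots, handling movement, aim, jump, damage and dual-wield firing.
; Interact line-traces for BPI_PickupInteractions actors, then spawns the weapon into the empty right (main) or left (offhand) arm as a timeline raises it.
; Equipped weapons are registered with the GameInstance.
; Switch swaps both weapons' attachments and references with a Niagara effect, mirroring the swap in the GameInstance.
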(event Custom|Anim_RarmSpawn
  (bind _armr (Variables|Default|GetArmR))
  (bind _relativelocation (Variables|/Script/Engine.SceneComponent|GetRelativeLocation _armr))
  (bind _movement (Timeline|Timeline_1 PlayFromStart)
    (:Update
      (Transformation|SetRelativeLocation _armr (Math|Vector|MakeVector (.x _relativelocation) (.y _relativelocation) (Math|Float|Lerp -45.0 -2e+01 _movement)) false false))))

(event Custom|Anim_LarmSpawn
  (bind _arml (Variables|Default|GetArmL))
  (bind _relativelocation (Variables|/Script/Engine.SceneComponent|GetRelativeLocation _arml))
  (bind _movement (Timeline|Timeline PlayFromStart)
    (:Update
      (Transformation|SetRelativeLocation _arml (Math|Vector|MakeVector (.x _relativelocation) (.y _relativelocation) (Math|Float|Lerp -45.0 -2e+01 _movement)) false false))))

(event Input|EnhancedActionEvents|EnhancedInputActionIA_Move
  (params (ActionValue :type Vector%202D%20Structure) (ElapsedSeconds :type Float%20%28double-precision%29) (TriggeredSeconds :type Float%20%28double-precision%29) (InputAction :type Input%20Action%20Object%20Reference :default "/Game/Input/IA_Move.IA_Move"))
  (Pawn|Input|AddMovementInput (Transformation|GetActorForwardVector) (.y ActionValue) false)
  (Pawn|Input|AddMovementInput (Transformation|GetActorRightVector) (.x ActionValue) false))

(event Input|EnhancedActionEvents|EnhancedInputActionIA_Aim
  (params (ActionValue :type Vector%202D%20Structure) (ElapsedSeconds :type Float%20%28double-precision%29) (TriggeredSeconds :type Float%20%28double-precision%29) (InputAction :type Input%20Action%20Object%20Reference :default "/Game/Input/IA_Aim.IA_Aim"))
  (Pawn|Input|AddControllerYawInput (* (.x ActionValue) 0.8))
  (Pawn|Input|AddControllerPitchInput (* (.y ActionValue) 0.8)))

(event Input|EnhancedActionEvents|EnhancedInputActionIA_Jump
  (params (ActionValue :type Boolean) (ElapsedSeconds :type Float%20%28double-precision%29) (TriggeredSeconds :type Float%20%28double-precision%29) (InputAction :type Input%20Action%20Object%20Reference :default "/Game/Input/IA_Jump.IA_Jump"))
  (:Started
    (Character|Jump)))

(event Input|EnhancedActionEvents|EnhancedInputActionIA_Fire
  (params (ActionValue :type Boolean) (ElapsedSeconds :type Float%20%28double-precision%29) (TriggeredSeconds :type Float%20%28double-precision%29) (InputAction :type Input%20Action%20Object%20Reference :default "/Game/Input/IA_Fire.IA_Fire"))
  (bind _a_mainhand (Variables|Default|GetA_MainHand))
  (:Triggered
    (if (Variables|Default|GetbCanFire)
      (Class|BPIWeaponInteractions|AllFire(Message) _a_mainhand)))
  (:Completed
    (Class|BPIWeaponInteractions|AllStopFire(Message) _a_mainhand)))

(event Input|EnhancedActionEvents|EnhancedInputActionIA_Interact
  (params (ActionValue :type Boolean) (ElapsedSeconds :type Float%20%28double-precision%29) (TriggeredSeconds :type Float%20%28double-precision%29) (InputAction :type Input%20Action%20Object%20Reference :default "/Game/Input/IA_Interact.IA_Interact"))
  (:Started
    (if (Variables|Default|GetbCanPickup)
      (bind _outhit (Utilities|LineTrace 2e+02)
        (:Success
          (if (Utilities|DoesObjectImplementInterface (.HitActor (Collision|BreakHitResult _outhit)) "/Game/Framework/Interfaces/BPI_PickupInteractions.BPI_PickupInteractions_C")
            (bind (_topickup _size _weaponenum) (Class|BPIPickupInteractions|Pickup(Message) (.HitActor (Collision|BreakHitResult _outhit))))
            (if (not (Utilities|IsValid (Variables|Default|GetA_MainHand)))
              (CallFunction|AnimRarmSpawn)
              (bind _returnvalue (CallFunction|SpawnMainSlot _topickup _size))
              (bind (_outcome _offhand_) (Utilities|SetNewActorValues _returnvalue (stale _returnvalue_2) :!label _label))
              (Default|SetNewEquipped (Variables|Default|GetBP_GI) _outcome _offhand_ _weaponenum)
              (Actor|DestroyActor (.HitActor (Collision|BreakHitResult _outhit)))
              (elif (not (Utilities|IsValid (Variables|Default|GetA_OffHand)))
                (CallFunction|AnimLarmSpawn)
                (bind _returnvalue_2 (CallFunction|SpawnOffHandSlot _topickup _size))
                (goto _label exeO)))))))))

(event Input|EnhancedActionEvents|EnhancedInputActionIA_Offhand
  (params (ActionValue :type Boolean) (ElapsedSeconds :type Float%20%28double-precision%29) (TriggeredSeconds :type Float%20%28double-precision%29) (InputAction :type Input%20Action%20Object%20Reference :default "/Game/Input/IA_Offhand.IA_Offhand"))
  (bind _a_offhand (Variables|Default|GetA_OffHand))
  (:Triggered
    (if (Variables|Default|GetbCanFire)
      (Class|BPIWeaponInteractions|AllFire(Message) _a_offhand)))
  (:Completed
    (Class|BPIWeaponInteractions|AllStopFire(Message) _a_offhand)))

(event Input|EnhancedActionEvents|EnhancedInputActionIA_Switch
  (params (ActionValue :type Boolean) (ElapsedSeconds :type Float%20%28double-precision%29) (TriggeredSeconds :type Float%20%28double-precision%29) (InputAction :type Input%20Action%20Object%20Reference :default "/Game/Input/IA_Switch.IA_Switch"))
  (:Started
    (Variables|Default|SetbCanFire false)
    (CallFunction|ArmSwitch)
    (Variables|Default|SetbCanFire true)))

(event EventBeginPlay
  (bind _asbp_game_instance (Utilities|Casting|CastToBP_GameInstance (Game|GetGameInstance)))
  (Variables|Default|SetBP_GI _asbp_game_instance)
  (bind _asbp_gpgm (Utilities|Casting|CastToBP_GPGM (Game|GetGameMode)))
  (Variables|Default|SetAs%20BP%20GPGM _asbp_gpgm))

(event Game|Damage|EventAnyDamage
  (params (Damage :type Float%20%28single-precision%29) (DamageType :type Damage%20Type%20Object%20Reference) (InstigatedBy :type Controller%20Object%20Reference) (DamageCauser :type Actor%20Object%20Reference))
  (Variables|Default|SetfHealth (- (Variables|Default|GetfHealth) Damage)))

(event EventOnLanded
  (params (Hit :type Hit%20Result%20Structure%20%28by%20ref%29))
  (Variables|/Script/Engine.CharacterMovementComponent|SetMaxWalkSpeed (Variables|Character|GetCharacterMovement) 7.5e+02))

(event EventPossessed
  (params (NewController :type Controller%20Object%20Reference))
  (bind _asbp_gppc (Utilities|Casting|CastToBP_GPPC NewController))
  (Variables|Default|SetAs%20BP%20GPPC _asbp_gppc))

(event EventOnJumped
  (Variables|/Script/Engine.CharacterMovementComponent|SetMaxWalkSpeed (Variables|Character|GetCharacterMovement) 825.0))

(fn ConstructionScript)

(fn SpawnMainSlot
  (params (Class :type BP%20Weapon%20Base%20Class%20Reference) (SpawnTransform_Scale :type Vector))
  (bind _self self)
  (bind _armr (Variables|Default|GetArmR))
  (bind _returnvalue (Game|SpawnActorfromClass Class (Math|Transform|MakeTransform (Transformation|GetWorldLocation _armr) (Transformation|GetWorldRotation _armr) SpawnTransform_Scale) "AlwaysSpawn" "MultiplyWithRoot" _self _self false _self))
  (Transformation|AttachComponentToComponent _returnvalue (Variables|Default|GetArmR) "None" "SnapToTarget" "SnapToTarget" "KeepRelative" true)
  (return _returnvalue))

(fn SpawnOffHandSlot
  (params (Class :type BP%20Weapon%20Base%20Class%20Reference) (SpawnTransform_Scale :type Vector))
  (bind _self self)
  (bind _arml (Variables|Default|GetArmL))
  (bind _returnvalue (Game|SpawnActorfromClass Class (Math|Transform|MakeTransform (Transformation|GetWorldLocation _arml) (Transformation|GetWorldRotation _arml) SpawnTransform_Scale) "AlwaysSpawn" "MultiplyWithRoot" _self _self true _self))
  (Transformation|AttachComponentToComponent _returnvalue (Variables|Default|GetArmL) "None" "SnapToTarget" "SnapToTarget" "KeepRelative" true)
  (return _returnvalue))

(fn ArmSwitch
  (Utilities|IsValid (Variables|Default|GetA_MainHand)
    (:Is%20Valid
      (Utilities|IsValid (Variables|Default|GetA_OffHand)
        (:Is%20Valid
          (Class|BPIWeaponInteractions|AllStopFire(Message) (Variables|Default|GetA_MainHand))
          (Class|BPIWeaponInteractions|AllStopFire(Message) (Variables|Default|GetA_OffHand))
          (Niagara|SpawnSystemAttached "/Game/Player/VFX/NS_WeaponSwitch.NS_WeaponSwitch" (Variables|/Game/Player/BP_WeaponBase.BP_WeaponBase_C|GetSpringArm (Variables|Default|GetA_MainHand)) "None" "0, 0, 0" "0, 0, 0" "SnapToTargetIncludingScale" true)
          (Niagara|SpawnSystemAttached "/Game/Player/VFX/NS_WeaponSwitch.NS_WeaponSwitch" (Variables|/Game/Player/BP_WeaponBase.BP_WeaponBase_C|GetSpringArm (Variables|Default|GetA_OffHand)) "None" "0, 0, 0" "0, 0, 0" "SnapToTargetIncludingScale" true)
          (Transformation|AttachComponentToComponent (Variables|Default|GetA_MainHand) (Variables|Default|GetArmL) "None" "SnapToTarget" "SnapToTarget" "SnapToTarget" true)
          (Transformation|AttachComponentToComponent (Variables|Default|GetA_OffHand) (Variables|Default|GetArmR) "None" "SnapToTarget" "SnapToTarget" "SnapToTarget" true)
          (LocalVariables|SetTemp_MainActor (Variables|Default|GetA_MainHand))
          (LocalVariables|SetTemp_OffHandActor (Variables|Default|GetA_OffHand))
          (Variables|Default|SetA_MainHand (LocalVariables|GetTemp_OffHandActor))
          (Variables|Default|SetA_OffHand (LocalVariables|GetTemp_MainActor))
          (Default|SwitchMain2OH (Variables|Default|GetBP_GI))
          (return))))))