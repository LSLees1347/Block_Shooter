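; Base Blueprint for player pickups that animates a static mesh and reports what it holds.
; On BeginPlay, rotating movement is bound to the mesh, and an optional Oscillation timeline bobs it with per-update vertical world offsets, replaying whenever it finishes forward.
; The Pickup function only returns the item to pick up, its size and its current count index, with no collection or destroy logic here.
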(event EventBeginPlay
  (Components|Movement|SetUpdatedComponent (Variables|Default|GetRotatingMovement) (Variables|Default|GetStaticMesh))
  (if (Variables|Default|GetbOscillate?)
    (bind (_direction _movement) (Timeline|Oscillation PlayFromStart)
      (:Update
        (Transformation|AddWorldOffset (Variables|Default|GetStaticMesh) (Math|Vector|MakeVector 0.0 0.0 (Math|Float|Lerp -0.2 0.2 _movement)) false false))
      (:Finished
        (switch Utilities|FlowControl|Switch|SwitchonETimelineDirection _direction
          (:Forward
            (Timeline|Oscillation PlayFromStart)))))))

(fn ConstructionScript)

(fn Pickup
  (return (Variables|Default|GetToPickUp) (Variables|Default|GetPickUpSize) (Variables|Default|GetCurrentIndex)))