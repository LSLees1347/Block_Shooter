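; BP_Crystal is a player crystal that launches from a crystal cluster and serves as a teleport point.
; FireCrystal alternates via FlipFlop between detaching it along the camera's forward vector with a Niagara flash, and teleporting the player to it.
; After teleporting, it snaps back onto the parent BP_CrystalCluster's spring arm with another flash.
; UnFireCrystal halts its movement and resets the DoOnce that gates each fire.
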(event EventBeginPlay
  (bind _asbp_player (Utilities|Casting|CastToBP_Player (Game|GetPlayerCharacter 0)))
  (Variables|Default|SetAs%20BP%20Player _asbp_player))

(event EventFireCrystal
  (bind _clusterref (Variables|Default|GetClusterREF))
  (Utilities|FlowControl|DoOnce false
    (:Completed
      (Utilities|FlowControl|FlipFlop
        (:A
          (Niagara|SpawnSystematLocation "/Game/AdvancedMagicFX13/Particles/Niagara/NS_ky_flash1.NS_ky_flash1" (Transformation|GetActorLocation))
          (Transformation|DetachFromActor "KeepWorld" "KeepWorld" "KeepWorld")
          (Variables|Default|SetbInCluster false)
          (Variables|/Script/Engine.MovementComponent|SetVelocity (Variables|Default|GetProjectileMovement) (* (Math|Vector|GetForwardVector (Variables|/Game/Player/BP_Player.BP_Player_C|GetCamera (Variables|Default|GetAs%20BP%20Player))) (Variables|Default|GetSpeed))))
        (:B
          (Variables|/Script/Engine.MovementComponent|SetVelocity (Variables|Default|GetProjectileMovement) "0, 0, 0")
          (Transformation|SetActorLocation (Variables|Default|GetAs%20BP%20Player) (Transformation|GetActorLocation) false false)
          (Utilities|IsValid _clusterref
            (:Is%20Valid
              (Transformation|AttachComponentToComponent (Variables|/Game/Player/BP_WeaponBase.BP_WeaponBase_C|GetSpringArm _clusterref) "None" "SnapToTarget" "SnapToTarget" "SnapToTarget" true)
              (Niagara|SpawnSystemAttached "/Game/AdvancedMagicFX13/Particles/Niagara/NS_ky_flash1.NS_ky_flash1" (Variables|Default|GetStaticMesh) "None" "0, 0, 0" "0, 0, 0" "SnapToTargetIncludingScale" true)
              (Variables|Default|SetbInCluster true))))))))

(event EventUnFireCrystal
  (bind _clusterref (Variables|Default|GetClusterREF))
  (Variables|/Script/Engine.MovementComponent|SetVelocity (Variables|Default|GetProjectileMovement) "0, 0, 0")
  (Utilities|FlowControl|DoOnce false) ; enters at Reset
)

(fn ConstructionScript
  (bind _asbp_crystal_cluster (Utilities|Casting|CastToBP_CrystalCluster (Actor|GetParentActor)))
  (Variables|Default|SetClusterREF _asbp_crystal_cluster))