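; BP_CrystalCluster is a player crystal cluster that grows to six crystals through upgrades.
; ApplyUpgrade fills the next child actor slot with BP_Crystal, increments the count and returns whether the cluster is full.
; The construction script gives the SpringArm a random rotation rate through RotatingMovement and also assigns it to Comp2Rot and Comp2Osi.
; AllFire and AllStopFire are empty, and the crystal fire message calls are unconnected.
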(event EventBeginPlay
  (|CallParentFunction)
  (Variables|Default|SetCrystalCount 0))

(event EventAllFire)

(event EventAllStopFire
  (params (Index :type Integer)))

(fn ConstructionScript
  (bind _rotatingmovement (Variables|Default|GetRotatingMovement))
  (bind _springarm (Variables|Default|GetSpringArm))
  (|CallParentFunction)
  (Variables|Default|SetComp2Rot _springarm)
  (Variables|Default|SetComp2Osi _springarm)
  (Components|Movement|SetUpdatedComponent _rotatingmovement _springarm)
  (Variables|/Script/Engine.RotatingMovementComponent|SetRotationRate _rotatingmovement (Math|Random|RandomRotator false)))

(fn ApplyUpgrade
  (params (Index :type Integer))
  (bind _crystalcount (Variables|Default|GetCrystalCount))
  (switch Utilities|FlowControl|Switch|SwitchonE_CrystalUpgrades (Utilities|Select :Index Index :Option%200 "NewEnumerator0" :Option%201 "NewEnumerator0")
    (:NewEnumerator0
      (ChildActorComponent|SetChildActorClass (Utilities|Select :Index (Variables|Default|GetCrystalCount) :Option%200 (Variables|Default|GetCrystal0) :Option%201 (Variables|Default|GetCrystal1) :Option%202 (Variables|Default|GetCrystal2) :Option%203 (Variables|Default|GetCrystal3) :Option%204 (Variables|Default|GetCrystal4) :Option%205 (Variables|Default|GetCrystal5)) "/Game/Player/Crystal/BP_Crystal.BP_Crystal_C")
      (Math|Integer|IncrementInt _crystalcount
        (:%20%20
          (return (>= _crystalcount 6)))))))