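; BP_Gun is the player's gun, with Fire branching to either a hitscan or projectile shot.
; Hitscan applies point damage from a passed hit result with a muzzle flash; projectile spawns BP_DefaultFire ahead of the player's GunStatic.
; Both paths re-enable the player's CanFire after PrimaryFireRate, using the player reference set by SetVAR.
; Projectile shots also play a shockwave and timeline-eased rotation through RotatingMovement.
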(event Custom|HitScanFire
  (params (Out%20Hit :type Hit%20Result%20Structure))
  (Utilities|FlowControl|Sequence
    (:then_0
      (Game|Damage|ApplyPointDamage (.HitActor (Collision|BreakHitResult Out%20Hit)) 1.0 (Transformation|GetActorLocation (Variables|Default|GetAs%20BP%20Player)) Out%20Hit (Pawn|GetController (Variables|Default|GetAs%20BP%20Player)) self)
      (Utilities|FlowControl|Delay (Variables|Default|GetPrimaryFireRate))
      (Variables|/Game/Player/BP_Player.BP_Player_C|SetbCanFire (Variables|Default|GetAs%20BP%20Player) true))
    (:then_1
      (Niagara|SpawnSystemAttached "/Game/Player/VFX/NS_MuzzleFlash.NS_MuzzleFlash" 0 "Muzzle" "0, 0, 0" "0.000000,-90.000000,0.000000" "SnapToTargetIncludingScale" true))))

(event Custom|FireAnimation
  (bind _rotation_rate_y (Variables|Default|GetRotation%20Rate%20Y))
  (Niagara|SpawnSystemAttached "/Game/Player/VFX/NS_Shockwave.NS_Shockwave" (Variables|Default|GetStaticMesh) "" "20.000000,0.000000,0.000000" "0.000000,0.000000,0.000000" "SnapToTarget" true)
  (Variables|/Script/Engine.RotatingMovementComponent|SetRotationRate (Variables|Default|GetRotatingMovement) (Math|Rotator|MakeRotator _rotation_rate_y 0.0 0.0))
  (bind _decel (Timeline|Firing PlayFromStart)
    (:Update
      (Variables|/Script/Engine.RotatingMovementComponent|SetRotationRate (Variables|Default|GetRotatingMovement) (Math|Rotator|MakeRotator (Math|Float|Lerp 6e+01 _rotation_rate_y _decel) 0.0 0.0)))))

(event Custom|ProjectileFire
  (bind _as_bp_player (Variables|Default|GetAs%20BP%20Player))
  (bind _as_bp_player_2 (Variables|Default|GetAs%20BP%20Player))
  (bind _gunstatic (Variables|/Game/Player/BP_Player.BP_Player_C|GetGunStatic _as_bp_player))
  (bind _returnvalue (Math|Vector|GetForwardVector _gunstatic))
  (Utilities|FlowControl|Sequence
    (:then_0
      (Game|SpawnActorfromClass "/Game/Player/Projectiles/BP_DefaultFire.BP_DefaultFire_C" (Math|Transform|MakeTransform (+ (Transformation|GetWorldLocation _gunstatic) (* (Math|Vector|GetForwardVector _gunstatic) 25.0)) (Math|Conversions|RotationFromXVector _returnvalue) "1.000000,1.000000,1.000000") "AlwaysSpawn" "MultiplyWithRoot" _as_bp_player_2 _returnvalue (Transformation|GetVelocity _as_bp_player) _as_bp_player_2)
      (Utilities|FlowControl|Delay (Variables|Default|GetPrimaryFireRate))
      (Variables|/Game/Player/BP_Player.BP_Player_C|SetbCanFire (Variables|Default|GetAs%20BP%20Player) true))
    (:then_1
      (CallFunction|FireAnimation))))

(event Custom|Fire
  (if (Variables|Default|GetbHitScanFire)
    (CallFunction|HitScanFire)
    (else
      (CallFunction|ProjectileFire))))

(fn ConstructionScript)

(fn SetVAR
  (params (As%20BP_Player :type BP%20Player%20Object%20Reference))
  (bind _output_get (Variables|Default|SetAs%20BP%20Player As%20BP_Player))
  (Variables|/Game/Player/BP_Player.BP_Player_C|SetbCanFire _output_get true)
  (return self))