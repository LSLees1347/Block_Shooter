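; BP_BulletBase is a base projectile for the player's BlockGun.
; On BeginPlay it sets its ProjectileMovement velocity from a direction vector scaled by Speed plus an added Velocity vector, then destroys itself after Duration.
; It also destroys itself on overlapping any actor other than its instigator, applying no damage here.
; A Niagara dash-fire spawn is present but unconnected.
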(event Collision|EventActorBeginOverlap
  (params (OtherActor :type Actor%20Object%20Reference))
  (if (not (== OtherActor (Game|GetInstigator)))
    (Actor|DestroyActor)))

(event EventBeginPlay
  (bind _speed (Variables|Default|GetSpeed))
  (Variables|/Script/Engine.MovementComponent|SetVelocity (Variables|Default|GetProjectileMovement) (+ (* (Variables|Default|GetFVector) (Math|Vector|MakeVector _speed _speed _speed)) (* (Variables|Default|GetVelocity) "1.000000,1.000000,1.000000")))
  (Utilities|FlowControl|Delay (Variables|Default|GetDuration))
  (Actor|DestroyActor))

(fn ConstructionScript)