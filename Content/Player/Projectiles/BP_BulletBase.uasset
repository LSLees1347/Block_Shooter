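; Base projectile actor for bullets under the player's projectiles, with movement and lifetime but no damage logic in its graph.
; On BeginPlay it sets the ProjectileMovement velocity from a direction vector scaled by Speed, plus the horizontal part of a stored Velocity.
; It destroys itself after Duration or on overlapping any actor other than its Instigator.
; A Niagara fire effect spawn is left unconnected and never runs.
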(event Collision|EventActorBeginOverlap
  (params (OtherActor :type Actor%20Object%20Reference))
  (if (not (== OtherActor (Game|GetInstigator)))
    (Actor|DestroyActor)))

(event EventBeginPlay
  (bind _speed (Variables|Default|GetSpeed))
  (Variables|/Script/Engine.MovementComponent|SetVelocity (Variables|Default|GetProjectileMovement) (+ (* (Variables|Default|GetFVector) (Math|Vector|MakeVector _speed _speed _speed)) (Math|Vector|MakeVector (.x (* (Variables|Default|GetVelocity) 1.0)) (.y (* (Variables|Default|GetVelocity) 1.0)) 0.0)))
  (Utilities|FlowControl|Delay (Variables|Default|GetDuration))
  (Actor|DestroyActor))

(fn ConstructionScript)