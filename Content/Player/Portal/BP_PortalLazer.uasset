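; Player-fired portal laser actor that renders a Niagara beam along the player's camera aim and damages what it hits.
; A looping timer runs a Visibility line trace from the camera, caching the hit location and applying damage plus sparks to actors with AC_Health.
; Tick sets the beam end to that hit, or to a point FRange ahead on a miss, although the trace uses its own hardcoded length.
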(event EventBeginPlay
  (Utilities|Time|SetTimerbyFunctionName 0 "Linetrace" 0.05 true)
  (Actor|Tick|SetActorTickEnabled true))

(event EventTick
  (params (DeltaSeconds :type Float%20%28single-precision%29))
  (bind _hitlocation (Variables|Default|GetHitLocation))
  (bind _asplayer (Variables|Default|GetAsPlayer))
  (bind _camera (Variables|/Game/Player/BP_Player.BP_Player_C|GetCamera _asplayer))
  (Niagara|SetNiagaraVariable(Vector3) (Variables|Default|GetNS_Beam) "Beam End" (Math|Vector|SelectVector (+ (* (Math|Vector|GetForwardVector _camera) (Variables|Default|GetfRange)) (Transformation|GetWorldLocation _camera)) _hitlocation (Utilities|Operators|EqualEqual :A _hitlocation :ErrorTolerance 1.0))))

(fn ConstructionScript)

(fn Linetrace
  (bind _asplayer (Variables|Default|GetAsPlayer))
  (bind _camera (Variables|/Game/Player/BP_Player.BP_Player_C|GetCamera _asplayer))
  (bind _returnvalue (Transformation|GetWorldLocation _camera))
  (bind (_outhit _returnvalue_2) (Collision|LineTraceByChannel _returnvalue (+ _returnvalue (* (Math|Vector|GetForwardVector _camera) 7.5e+02)) "TraceTypeQuery1" false (Utilities|Array|MakeArray (Game|GetInstigator) (Variables|Default|GetAsPlayer)) "None"))
  (if _returnvalue_2
    (Variables|Default|SetHitLocation (.Location (Collision|BreakHitResult _outhit)))
    (Utilities|IsValid (Actor|GetComponentbyClass (.HitActor (Collision|BreakHitResult _outhit)) "/Game/Components/AC_Health.AC_Health_C")
      (:Is%20Valid
        (Default|TakeDamage (Actor|GetComponentbyClass (.HitActor (Collision|BreakHitResult _outhit)) "/Game/Components/AC_Health.AC_Health_C") 1.0)
        (Niagara|SpawnSystematLocation "/Game/Player/Portal/NS_BeamSparks.NS_BeamSparks" (.Location (Collision|BreakHitResult _outhit)))
        (return))
      (:Is%20Not%20Valid
        _))
    (else
      (Variables|Default|SetHitLocation "0, 0, 0")))
  (return))