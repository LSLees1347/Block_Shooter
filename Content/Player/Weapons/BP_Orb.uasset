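; BP_Orb is an orb actor in the player's weapons set, with a mesh that spins and bobs in place.
; On BeginPlay, RotatingMovement targets the static mesh while a timeline, restarted each time it finishes, lerps the mesh's relative Z for a continuous hover.
; OrbSetVAR stores the owning player and offhand flag and returns the orb itself, while PortalSetVAR is an empty stub.
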(event EventBeginPlay
  (Components|Movement|SetUpdatedComponent (Variables|Default|GetRotatingMovement) (Variables|Default|GetStaticMesh))
  (bind _newtrack_0 (Timeline|Timeline PlayFromStart)
    (:Update
      (Transformation|SetRelativeLocation (Variables|Default|GetStaticMesh) (Math|Vector|MakeVector 0.0 0.0 (Math|Float|Lerp -5.0 5.0 _newtrack_0)) false false))
    (:Finished
      (Timeline|Timeline PlayFromStart))))

(fn ConstructionScript)

(fn OrbSetVAR
  (params (As%20BP_Player :type BP%20Player%20Object%20Reference) (bIsOffhand :type Boolean))
  (Variables|Default|SetAs%20BP%20Player As%20BP_Player)
  (Variables|Default|SetbIsOffHand bIsOffhand)
  (return self))

(fn PortalSetVAR
  (params (As%20BP_Player :type BP%20Player%20Object%20Reference) (bIsOffhand :type Boolean)))