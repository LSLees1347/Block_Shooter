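; Base player weapon, held in either hand, with a mesh that bobs on a looping timeline and rotates.
; AllFire spawns BP_DefaultFire along the matching arm's forward vector, gated by a fire-rate delay, then triggers a shockwave and decelerating spin.
; HitScanFire takes a supplied hit, applies point damage, shows muzzle flash and re-enables the player's CanFire after the delay.
; PortalSetVAR binds player and hand; OrbSetVAR is empty.
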(event Custom|HitScanFire
  (params (Out%20Hit :type Hit%20Result%20Structure))
  (Utilities|FlowControl|Sequence
    (:then_0
      (Game|Damage|ApplyPointDamage (.HitActor (Collision|BreakHitResult Out%20Hit)) 1.0 (Transformation|GetActorLocation (Variables|Default|GetAs%20BP%20Player)) Out%20Hit (Pawn|GetController (Variables|Default|GetAs%20BP%20Player)) self)
      (Utilities|FlowControl|Delay (Variables|Default|GetPrimaryFireRate))
      (Variables|/Game/Player/Primary/BP_Player.BP_Player_C|SetbCanFire (Variables|Default|GetAs%20BP%20Player) true))
    (:then_1
      (Niagara|SpawnSystemAttached "/Game/Player/VFX/NS_MuzzleFlash.NS_MuzzleFlash" 0 "Muzzle" "0, 0, 0" "0.000000,-90.000000,0.000000" "SnapToTargetIncludingScale" true))))

(event Custom|FireAnimation
  (bind _rotation_rate_y (Variables|Default|GetRotation%20Rate%20Y))
  (Niagara|SpawnSystemAttached "/Game/Player/VFX/NS_Shockwave.NS_Shockwave" (Variables|Default|GetStaticMesh) "" "0, 0, 0" "0, 0, 0" "SnapToTarget" true)
  (Variables|/Script/Engine.RotatingMovementComponent|SetRotationRate (Variables|Default|GetRotatingMovement) (Math|Rotator|MakeRotator _rotation_rate_y 0.0 0.0))
  (bind _decel (Timeline|Firing PlayFromStart)
    (:Update
      (Variables|/Script/Engine.RotatingMovementComponent|SetRotationRate (Variables|Default|GetRotatingMovement) (Math|Rotator|MakeRotator (Math|Float|Lerp 3e+01 _rotation_rate_y _decel) 0.0 0.0)))))

(event EventBeginPlay
  (bind _osillationamount (Variables|Default|GetOsillationAmount))
  (Components|Movement|SetUpdatedComponent (Variables|Default|GetRotatingMovement) (Variables|Default|GetStaticMesh))
  (bind _newtrack_0 (Timeline|Timeline PlayFromStart)
    (:Update
      (Transformation|SetRelativeLocation (Variables|Default|GetStaticMesh) (Math|Vector|MakeVector 0.0 0.0 (Math|Float|Lerp (* _osillationamount -1.0) _osillationamount _newtrack_0)) false false))
    (:Finished
      (Timeline|Timeline PlayFromStart))))

(event EventAllFire
  (bind _as_bp_player (Variables|Default|GetAs%20BP%20Player))
  (bind _as_bp_player_2 (Variables|Default|GetAs%20BP%20Player))
  (bind _bisoffhand (Variables|Default|GetbIsOffHand))
  (bind _arml (Variables|/Game/Player/Primary/BP_Player.BP_Player_C|GetArmL _as_bp_player))
  (bind _armr (Variables|/Game/Player/Primary/BP_Player.BP_Player_C|GetArmR _as_bp_player))
  (bind _returnvalue (select _bisoffhand _arml _armr))
  (bind _returnvalue_2 (Math|Vector|GetForwardVector _returnvalue))
  (if (Variables|Default|GetbCanFire)
    (Variables|Default|SetbCanFire false)
    (Utilities|FlowControl|Sequence
      (:then_0
        (Game|SpawnActorfromClass "/Game/Player/Projectiles/BP_DefaultFire.BP_DefaultFire_C" (Math|Transform|MakeTransform (+ (Transformation|GetActorLocation) (* (Transformation|GetActorForwardVector) 25.0)) (Math|Conversions|RotationFromXVector _returnvalue_2) "1.000000,1.000000,1.000000") "AlwaysSpawn" "MultiplyWithRoot" _as_bp_player_2 _returnvalue_2 (Transformation|GetVelocity _as_bp_player) _as_bp_player_2)
        (Utilities|FlowControl|Delay (Variables|Default|GetPrimaryFireRate))
        (Variables|Default|SetbCanFire true))
      (:then_1
        (CallFunction|FireAnimation)))))

(fn ConstructionScript)

(fn OrbSetVAR
  (params (As%20BP_Player :type BP%20Player%20Object%20Reference) (bIsOffhand :type Boolean))
  (return 0))

(fn PortalSetVAR
  (params (As%20BP_Player :type BP%20Player%20Object%20Reference) (bIsOffhand :type Boolean))
  (bind _output_get (Variables|Default|SetAs%20BP%20Player As%20BP_Player))
  (Variables|/Game/Player/Primary/BP_Player.BP_Player_C|SetbCanFire _output_get true)
  (Variables|Default|SetbIsOffHand bIsOffhand)
  (return self))