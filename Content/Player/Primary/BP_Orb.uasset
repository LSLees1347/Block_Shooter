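; BP_Orb is an orb actor in the player's primary set that spins and bobs up and down.
; On BeginPlay, RotatingMovement drives the static mesh while a self-restarting timeline lerps the actor's relative Z through a small range.
; OrbSetVAR stores the player reference and returns the orb itself; the other SetVAR functions are empty stubs.
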(event EventBeginPlay
  (Components|Movement|SetUpdatedComponent (Variables|Default|GetRotatingMovement) (Variables|Default|GetStaticMesh))
  (bind _movement (Timeline|Timeline PlayFromStart)
    (:Update
      (Transformation|SetActorRelativeLocation (Math|Vector|MakeVector 0.0 0.0 (Math|Float|Lerp -5.0 5.0 _movement))))
    (:Finished
      (Timeline|Timeline PlayFromStart))))

(fn ConstructionScript)

(fn ASetVAR
  (params (Player :type BP%20Player%20Object%20Reference) (ToOut :type E_AllPickups%20Enum :default "NewEnumerator4"))
  (return 0 0 0))

(fn GunSetVAR
  (params (As%20BP_Player :type BP%20Player%20Object%20Reference)))

(fn OrbSetVAR
  (params (As%20BP_Player :type BP%20Player%20Object%20Reference))
  (Variables|Default|SetAs%20BP%20Player As%20BP_Player)
  (return self))

(fn UpgradesSetVAR
  (params (As%20BP_Player :type BP%20Player%20Object%20Reference))
  (return 0))