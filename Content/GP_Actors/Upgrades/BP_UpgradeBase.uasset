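; BP_UpgradeBase is the base actor for upgrade pickups, displaying a mesh that spins through RotatingMovement and optionally bobs vertically via a looping Timeline.
; ScrollUpgrade moves the selected index within a clamped range, and AddMaxedUpgrade records indices of maxed upgrades.
; SelectUpgrade returns the target weapon and the current index.
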(event EventAddMaxedUpgrade
  (params (Index :type Integer))
  (Utilities|Array|Add (Variables|Default|GetAll_MaxedUpgrades) Index))

(event EventBeginPlay
  (if (Variables|Default|GetbOscillate?)
    (bind _newtrack_0 (Timeline|Timeline PlayFromStart)
      (:Update
        (Transformation|SetRelativeLocation (Variables|Default|GetStaticMesh) (Math|Vector|MakeVector 0.0 0.0 (Math|Float|Lerp -12.0 12.0 _newtrack_0)) false false))
      (:Finished
        (Timeline|Timeline PlayFromStart)))))

(event EventScrollUpgrade
  (params (ScrollAmount :type Integer))
  (Variables|Default|SetUpgradeIndex (Math|Integer|Clamp(Integer) (+ (Variables|Default|GetUpgradeIndex) ScrollAmount) 0 (Variables|Default|GetIndexTotal))))

(fn ConstructionScript
  (Components|Movement|SetUpdatedComponent (Variables|Default|GetRotatingMovement) (Variables|Default|GetStaticMesh)))

(fn SelectUpgrade
  (return (Variables|Default|GetForWeapon) (Variables|Default|GetUpgradeIndex)))