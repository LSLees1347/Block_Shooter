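; BP_StationBase is a base weapon station actor with a rotating, optionally bobbing mesh and a selection widget shown while the player overlaps its hitbox.
; StationData initializes the widget and supplies the upgrade map whose values cap each inventory slot.
; ScrollIndex moves the clamped selection once the first slot is non-zero.
; SelectIndex increments the selected slot unless maxed, refreshes the widget, and returns class, spawn size, index and maxed state.
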(event OnComponentBeginOverlap(WidgetHitbox)
  (params (OverlappedComponent :type Primitive%20Component%20Object%20Reference) (OtherActor :type Actor%20Object%20Reference) (OtherComp :type Primitive%20Component%20Object%20Reference) (OtherBodyIndex :type Integer) (bFromSweep :type Boolean) (SweepResult :type Hit%20Result%20Structure%20%28by%20ref%29))
  (Utilities|Casting|CastToBP_Player OtherActor)
  (Rendering|SetVisibility (Variables|Default|GetWidget) true false))

(event OnComponentEndOverlap(WidgetHitbox)
  (params (OverlappedComponent :type Primitive%20Component%20Object%20Reference) (OtherActor :type Actor%20Object%20Reference) (OtherComp :type Primitive%20Component%20Object%20Reference) (OtherBodyIndex :type Integer))
  (Utilities|Casting|CastToBP_Player OtherActor)
  (Rendering|SetVisibility (Variables|Default|GetWidget) false false))

(event EventBeginPlay
  (bind _aswbp_station (Utilities|Casting|CastToWBP_Station (UserInterface|GetWidget (Variables|Default|GetWidget))))
  (bind _output_get (Variables|Default|SetWBP_Station _aswbp_station))
  (Default|Init _output_get (Variables|Default|GetStationData))
  (Components|Movement|SetUpdatedComponent (Variables|Default|GetRotatingMovement) (Variables|Default|GetStaticMesh))
  (if (Variables|Default|GetbOscillate?)
    (bind _newtrack_0 (Timeline|Timeline PlayFromStart)
      (:Update
        (Transformation|SetRelativeLocation (Variables|Default|GetStaticMesh) (Math|Vector|MakeVector 0.0 0.0 (Math|Float|Lerp -12.0 12.0 _newtrack_0)) false false)
        (Transformation|SetRelativeLocation (Variables|Default|GetWidget) (Math|Vector|MakeVector 0.0 0.0 (+ (Math|Float|Lerp -12.0 12.0 _newtrack_0) 35.0)) false false))
      (:Finished
        (Timeline|Timeline PlayFromStart)))))

(event EventScrollIndex
  (params (Input :type Integer))
  (if (not (== (Utilities|Array|Get(acopy) (Variables|Default|GetInventory)) 0))
    (bind _output_get (Variables|Default|SetSelection (Math|Integer|Clamp(Integer) (+ Input (Variables|Default|GetSelection)) 0 (- (Utilities|Map|Length (Variables|/Game/Data/PDA_Base.PDA_Base_C|GetRO_UpgradeMap (Variables|Default|GetStationData))) 1))))
    (CallFunction|CheckMaxed)
    (Default|UpdateSelection (Variables|Default|GetWBP_Station) _output_get (Variables|Default|GetInventory))))

(fn ConstructionScript)

(fn CheckMaxed
  (bind _selection (Variables|Default|GetSelection))
  (bind _values (Utilities|Map|Values (Variables|/Game/Data/PDA_Base.PDA_Base_C|GetRO_UpgradeMap (Variables|Default|GetStationData))))
  (Math|Integer|CompareInt (Utilities|Array|Get(acopy) (Variables|Default|GetInventory) _selection) (Utilities|Array|Get(acopy) _values _selection)
    (:>
      (Variables|Default|SetSelectionMaxed? true :!label _label))
    (:==
      (goto _label))
    (:<
      (Variables|Default|SetSelectionMaxed? false)))
  (return))

(fn SelectIndex
  (CallFunction|CheckMaxed)
  (if (Variables|Default|GetSelectionMaxed?)
    _
    (else
      (Math|Integer|IncrementInt (Utilities|Array|Get(acopy) (Variables|Default|GetInventory) (Variables|Default|GetSelection))
        (:%20%20
          (Default|UpdateSelection (Variables|Default|GetWBP_Station) (Variables|Default|GetSelection) (Variables|Default|GetInventory))))))
  (return (Variables|/Game/Data/PDA_Base.PDA_Base_C|GetClass (Variables|Default|GetStationData)) (Variables|Default|GetSpawnSize) (Variables|Default|GetSelection) (Variables|Default|GetSelectionMaxed?)))