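; BP_PickupBase is a base pickup actor that spins its static mesh and can bob it up and down in the world.
; On BeginPlay it points RotatingMovement at the mesh and, if Oscillate is set, replays a timeline that lerps the mesh's relative Z around its origin.
; The Pickup function only returns the item to pick up, its size and the current count index, without changing or destroying the actor.
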(event EventBeginPlay
  (Components|Movement|SetUpdatedComponent (Variables|Default|GetRotatingMovement) (Variables|Default|GetStaticMesh))
  (if (Variables|Default|GetbOscillate?)
    (bind _newtrack_0 (Timeline|Timeline PlayFromStart)
      (:Update
        (Transformation|SetRelativeLocation (Variables|Default|GetStaticMesh) (Math|Vector|MakeVector 0.0 0.0 (Math|Float|Lerp -12.0 12.0 _newtrack_0)) false false))
      (:Finished
        (Timeline|Timeline PlayFromStart)))))

(fn ConstructionScript)

(fn Pickup
  (return (Variables|Default|GetToPickUp) (Variables|Default|GetPickUpSize) (Variables|Default|GetCurrentIndex)))