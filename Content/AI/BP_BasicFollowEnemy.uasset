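; BP_BasicFollowEnemy is an enemy that moves toward the player and awards score when it dies.
; On BeginPlay its AI controller issues a single SimpleMoveToActor with the player controller, rather than the pawn, as goal, then caches the controlled BP_Player.
; When its HealthComponent fires OnDeath, it adds its Value to the cached player's ScoreComponent and destroys itself.
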(event OnDeath(HealthComponent)
  (Default|AddScore (Variables|/Game/Player/BP_Player.BP_Player_C|GetScore%20Component (Variables|Default|GetAs%20BP%20Player)) (Variables|Default|GetValue))
  (Actor|DestroyActor))

(event EventBeginPlay
  (bind _returnvalue (Game|GetPlayerController 0))
  (AI|Navigation|SimpleMovetoActor (AI|GetAIController self) _returnvalue)
  (bind _asbp_player (Utilities|Casting|CastToBP_Player (Pawn|GetControlledPawn _returnvalue)))
  (Variables|Default|SetAs%20BP%20Player _asbp_player))

(fn ConstructionScript)