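; BP_GPPC is a Player Controller that sets up input and the HUD for the local player.
; On BeginPlay, if the Enhanced Input subsystem is valid, it adds IMC_Main, shows the HUD, switches to game-only input and hides the mouse cursor.
; UIShowHUD creates WBP_HUD only when no valid instance is stored, then adds it to the viewport.
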(event EventBeginPlay
  (bind _returnvalue (PlayerController|LocalPlayerSubsystems|GetEnhancedInputLocalPlayerSubsystem))
  (Utilities|IsValid _returnvalue
    (:Is%20Valid
      (Input|AddMappingContext _returnvalue "/Game/Input/IMC_Main.IMC_Main" 0 "(bIgnoreAllPressedKeysUntilRelease=True,bForceImmediately=False,bNotifyUserSettings=False)")
      (CallFunction|UIShowHUD)
      (Input|SetInputModeGameOnly self false)
      (Variables|Default|SetbShowMouseCursor false))))

(fn ConstructionScript)

(fn UIShowHUD
  (Utilities|IsValid (Variables|Default|GetWBP_HUD)
    (:Is%20Valid
      _)
    (:Is%20Not%20Valid
      (bind _returnvalue (UserInterface|CreateWidget "/Game/Widgets/WBP_HUD.WBP_HUD_C" self))
      (Variables|Default|SetWBP_HUD _returnvalue)))
  (UserInterface|Viewport|AddtoViewport (Variables|Default|GetWBP_HUD) 0)
  (return))