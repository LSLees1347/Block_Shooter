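; BP_WeaponBase is a base weapon Blueprint that provides optional spin and bobbing motion for designated components.
; On BeginPlay, RotatingMovement drives Comp2Rot if it is valid.
; If Comp2Osi is valid, a self-restarting Timeline lerps its relative Z between negative and positive FOssilationAmount.
; SetVAR and ApplyUpgrade are empty stubs, and the construction script does nothing.
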(event EventBeginPlay
  (bind _fossilationamount (Variables|Default|GetfOssilationAmount))
  (Utilities|IsValid (Variables|Default|GetComp2Rot)
    (:Is%20Valid
      (Components|Movement|SetUpdatedComponent (Variables|Default|GetRotatingMovement) (Variables|Default|GetComp2Rot)))
    (:Is%20Not%20Valid
      _))
  (Utilities|IsValid (Variables|Default|GetComp2Osi)
    (:Is%20Valid
      (bind _newtrack_0 (Timeline|Timeline PlayFromStart)
        (:Update
          (Transformation|SetRelativeLocation (Variables|Default|GetComp2Osi) (Math|Vector|MakeVector 0.0 0.0 (Math|Float|Lerp (* _fossilationamount -1.0) _fossilationamount _newtrack_0)) false false))
        (:Finished
          (Timeline|Timeline PlayFromStart))))))

(fn ConstructionScript)

(fn SetVAR
  (return))

(fn ApplyUpgrade
  (params (Index :type Integer))
  (return))