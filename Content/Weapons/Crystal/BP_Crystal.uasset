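; BP_Crystal is a player weapon crystal that grows in on spawn, then can be launched as a damaging projectile.
; On spawn it attaches an effect, plays a scale timeline and sets CanFire after a short delay.
; FireCrystal sends it along the player camera's forward vector and destroys it after a timeout.
; Overlapping an Enemy-tagged actor applies damage through AC_Health, then shares the hit effect and destroy path with its own death.
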(event OnDeath(AC_Health)
  (Niagara|SpawnSystematLocation "/Game/AdvancedMagicFX12/particles/Niagara/NS_ky_hit_fire.NS_ky_hit_fire" (Transformation|GetActorLocation))
  (Actor|DestroyActor))

(event EventBeginPlay
  (bind _asbp_player (Utilities|Casting|CastToBP_Player (Game|GetPlayerCharacter 0)))
  (Variables|Default|SetAs%20BP%20Player _asbp_player)
  (Niagara|SpawnSystemAttached 0 (Variables|Default|GetStaticMesh) "None" "0, 0, 0" "0, 0, 0" "SnapToTargetIncludingScale" true)
  (Utilities|FlowControl|Sequence
    (:then_0
      (Utilities|FlowControl|Delay 1.5)
      (Variables|Default|SetCanFire true))
    (:then_1
      (bind _scale_3d (Timeline|Scale PlayFromStart)
        (:Update
          (Transformation|SetActorScale3D (Math|Vector|MakeVector _scale_3d _scale_3d _scale_3d)))))))

(event Collision|EventActorBeginOverlap
  (params (OtherActor :type Actor%20Object%20Reference))
  (if (Actor|ActorHasTag OtherActor "Enemy")
    (Default|TakeDamage (Actor|GetComponentbyClass OtherActor "/Game/Components/AC_Health.AC_Health_C") (Variables|Default|GetDamage))
    (Niagara|SpawnSystematLocation "/Game/AdvancedMagicFX12/particles/Niagara/NS_ky_hit_fire.NS_ky_hit_fire" (Transformation|GetActorLocation))
    (Actor|DestroyActor)))

(event EventFireCrystal
  (Niagara|SpawnSystematLocation "/Game/AdvancedMagicFX13/Particles/Niagara/NS_ky_flash1.NS_ky_flash1" (Transformation|GetActorLocation))
  (Variables|/Script/Engine.MovementComponent|SetVelocity (Variables|Default|GetProjectileMovement) (* (Math|Vector|GetForwardVector (Variables|/Game/Player/BP_Player.BP_Player_C|GetCamera (Variables|Default|GetAs%20BP%20Player))) (Variables|Default|GetSpeed)))
  (Utilities|FlowControl|Delay 2.5)
  (Actor|DestroyActor))

(fn ConstructionScript)