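; BP_CrystalCluster is a weapon holding up to six BP_Crystal child actors on a rotating spring arm.
; ApplyUpgrade activates further crystal slots and their Niagara effects, with the CryStatus map tracking which are loaded.
; FireTick detaches and fires the first loaded crystal once until EndFire resets it.
; ReloadTick blocks firing until EndReload and respawns spent crystals on a delay, only when slot 0's actor is invalid.
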(event EventBeginPlay
  (|CallParentFunction)
  (Utilities|Map|Add (Variables|Default|GetCry_Status) (Variables|Default|GetCrystal0) true)
  (Math|Integer|IncrementInt (Variables|Default|GetCrystalCount)))

(event EventApplyUpgrade
  (params (Index :type Integer))
  (bind _crystal0 (Variables|Default|GetCrystal0))
  (bind _crystal1 (Variables|Default|GetCrystal1))
  (bind _crystal2 (Variables|Default|GetCrystal2))
  (bind _crystal3 (Variables|Default|GetCrystal3))
  (bind _crystal4 (Variables|Default|GetCrystal4))
  (bind _crystal5 (Variables|Default|GetCrystal5))
  (bind _crystalcount (Variables|Default|GetCrystalCount))
  (bind _returnvalue (Utilities|Select :Index _crystalcount :Option%200 _crystal0 :Option%201 _crystal1 :Option%202 _crystal2 :Option%203 _crystal3 :Option%204 _crystal4 :Option%205 _crystal5))
  (switch int Index
    (:1
      (ChildActorComponent|SetChildActorClass _returnvalue "/Game/Weapons/Crystal/BP_Crystal.BP_Crystal_C")
      (Rendering|SetVisibility (Utilities|Select :Index (Variables|Default|GetCrystalCount) :Option%200 (Variables|Default|GetNiagara0) :Option%201 (Variables|Default|GetNiagara1) :Option%202 (Variables|Default|GetNiagara2) :Option%203 (Variables|Default|GetNiagara3) :Option%204 (Variables|Default|GetNiagara4) :Option%205 (Variables|Default|GetNiagara5)) true false)
      (Utilities|Map|Add (Variables|Default|GetCry_Status) _returnvalue true)
      (Math|Integer|IncrementInt (Variables|Default|GetCrystalCount)))))

(event EventFireTick
  (if (Variables|Default|GetCanClusterFire)
    (Utilities|FlowControl|DoOnce false
      (:Completed
        (bind _values (Utilities|Map|Values (Variables|Default|GetCry_Status)))
        (if (not (< (Utilities|Array|FindItem _values true) 0))
          (bind _asbp_crystal (Utilities|Casting|CastToBP_Crystal (Utilities|Select :Index (Utilities|Array|FindItem _values true) :Option%200 (Variables|/Script/Engine.ChildActorComponent|GetChildActor (Variables|Default|GetCrystal0)) :Option%201 (Variables|/Script/Engine.ChildActorComponent|GetChildActor (Variables|Default|GetCrystal1)) :Option%202 (Variables|/Script/Engine.ChildActorComponent|GetChildActor (Variables|Default|GetCrystal2)) :Option%203 (Variables|/Script/Engine.ChildActorComponent|GetChildActor (Variables|Default|GetCrystal3)) :Option%204 (Variables|/Script/Engine.ChildActorComponent|GetChildActor (Variables|Default|GetCrystal4)) :Option%205 (Variables|/Script/Engine.ChildActorComponent|GetChildActor (Variables|Default|GetCrystal5)))))
          (if (Variables|/Game/Weapons/Crystal/BP_Crystal.BP_Crystal_C|GetCanFire _asbp_crystal)
            (Transformation|DetachFromActor (Utilities|Select :Index (Utilities|Array|FindItem _values true) :Option%200 (Variables|/Script/Engine.ChildActorComponent|GetChildActor (Variables|Default|GetCrystal0)) :Option%201 (Variables|/Script/Engine.ChildActorComponent|GetChildActor (Variables|Default|GetCrystal1)) :Option%202 (Variables|/Script/Engine.ChildActorComponent|GetChildActor (Variables|Default|GetCrystal2)) :Option%203 (Variables|/Script/Engine.ChildActorComponent|GetChildActor (Variables|Default|GetCrystal3)) :Option%204 (Variables|/Script/Engine.ChildActorComponent|GetChildActor (Variables|Default|GetCrystal4)) :Option%205 (Variables|/Script/Engine.ChildActorComponent|GetChildActor (Variables|Default|GetCrystal5))) "KeepWorld" "KeepWorld" "KeepWorld")
            (Class|BPICrystalInteractions|FireCrystal(Message) (Utilities|Select :Index (Utilities|Array|FindItem _values true) :Option%200 (Variables|/Script/Engine.ChildActorComponent|GetChildActor (Variables|Default|GetCrystal0)) :Option%201 (Variables|/Script/Engine.ChildActorComponent|GetChildActor (Variables|Default|GetCrystal1)) :Option%202 (Variables|/Script/Engine.ChildActorComponent|GetChildActor (Variables|Default|GetCrystal2)) :Option%203 (Variables|/Script/Engine.ChildActorComponent|GetChildActor (Variables|Default|GetCrystal3)) :Option%204 (Variables|/Script/Engine.ChildActorComponent|GetChildActor (Variables|Default|GetCrystal4)) :Option%205 (Variables|/Script/Engine.ChildActorComponent|GetChildActor (Variables|Default|GetCrystal5))))
            (Utilities|Map|Add (Variables|Default|GetCry_Status) (Utilities|Select :Index (Utilities|Array|FindItem _values true) :Option%200 (Variables|Default|GetCrystal0) :Option%201 (Variables|Default|GetCrystal1) :Option%202 (Variables|Default|GetCrystal2) :Option%203 (Variables|Default|GetCrystal3) :Option%204 (Variables|Default|GetCrystal4) :Option%205 (Variables|Default|GetCrystal5)) false)))))))

(event EventEndFire
  (Utilities|FlowControl|DoOnce false) ; enters at Reset
)

(event EventEndReload
  (Variables|Default|SetCanClusterFire true))

(event EventReloadTick
  (Variables|Default|SetCanClusterFire false)
  (Utilities|FlowControl|DoOnce false :!label _label
    (:Completed
      (bind _values (Utilities|Map|Values (Variables|Default|GetCry_Status)))
      (if (< (Utilities|Array|FindItem _values false) 0)
        (Utilities|FlowControl|Delay 0.2)
        (goto _label Reset)
        (else
          (Utilities|IsValid (Utilities|Select :Index 0 :Option%200 (Variables|/Script/Engine.ChildActorComponent|GetChildActor (Variables|Default|GetCrystal0)) :Option%201 (Variables|/Script/Engine.ChildActorComponent|GetChildActor (Variables|Default|GetCrystal1)) :Option%202 (Variables|/Script/Engine.ChildActorComponent|GetChildActor (Variables|Default|GetCrystal2)) :Option%203 (Variables|/Script/Engine.ChildActorComponent|GetChildActor (Variables|Default|GetCrystal3)) :Option%204 (Variables|/Script/Engine.ChildActorComponent|GetChildActor (Variables|Default|GetCrystal4)) :Option%205 (Variables|/Script/Engine.ChildActorComponent|GetChildActor (Variables|Default|GetCrystal5)))
            (:Is%20Valid
              (goto _label Reset))
            (:Is%20Not%20Valid
              (ChildActorComponent|SetChildActorClass (Utilities|Select :Index (Utilities|Array|FindItem _values false) :Option%200 (Variables|Default|GetCrystal0) :Option%201 (Variables|Default|GetCrystal1) :Option%202 (Variables|Default|GetCrystal2) :Option%203 (Variables|Default|GetCrystal3) :Option%204 (Variables|Default|GetCrystal4) :Option%205 (Variables|Default|GetCrystal5)) "/Game/Weapons/Crystal/BP_Crystal.BP_Crystal_C")
              (Utilities|Map|Add (Variables|Default|GetCry_Status) (Utilities|Select :Index (Utilities|Array|FindItem _values false) :Option%200 (Variables|Default|GetCrystal0) :Option%201 (Variables|Default|GetCrystal1) :Option%202 (Variables|Default|GetCrystal2) :Option%203 (Variables|Default|GetCrystal3) :Option%204 (Variables|Default|GetCrystal4) :Option%205 (Variables|Default|GetCrystal5)) true)
              (Utilities|FlowControl|Delay 0.5)
              (goto _label Reset))))))))

(fn ConstructionScript
  (bind _springarm (Variables|Default|GetSpringArm))
  (|CallParentFunction)
  (Variables|Default|SetComp2Rot _springarm)
  (Variables|Default|SetComp2Osi _springarm)
  (Components|Movement|SetUpdatedComponent (Variables|Default|GetRotatingMovement) _springarm))